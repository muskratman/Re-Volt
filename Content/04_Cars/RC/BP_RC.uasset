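; RC car Blueprint that sets its handling values and hooks up respawning when play starts.
; BeginPlay sets steering, four-wheel drive, speed and throttle variables, then binds Respawn to the destruction of player 0's pawn.
; Respawn casts to InGame_PlayerController and calls its Respawn.
; Alternative tunings (including Junior RC), mass and center-of-mass overrides, and physics debug commands remain as disconnected nodes.
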(event `self.ReceiveBeginPlay`
  (set `self.Steer_Angle_Max` 30.0)
  (set `self.4WD` true)
  (set `self.Max_Speed` 60.0)
  (set `self.Throttle_Max` 100.0)
  (set `self.Steer_Change_Speed` 3.0)
  ;[1 0.3105 0.3603] RESPAWN
  (add `Actor.OnDestroyed` (`GameplayStatics.GetPlayerPawn` 0) (delegate `Respawn`)))

(event `Respawn`
  (params (DestroyedActor :type "Actor Object Reference"))
  ;[1 0.3105 0.3603] RESPAWN
  (bind _asin_game_player_controller (cast `/Game/00_InGame/InGame_PlayerController` (`GameplayStatics.GetPlayerController` 0)))
  (`/Game/00_InGame/InGame_PlayerController.Respawn` _asin_game_player_controller))

(fn `UserConstructionScript`
  (`parent.UserConstructionScript`))