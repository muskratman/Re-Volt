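; Player-drivable car Blueprint on SimpleWheeledVehicleMovement, with speed-curve steering, capped front or four-wheel drive and a rear handbrake.
; Negative throttle briefly pulses the rear brakes instead of reversing.
; The spring-arm camera orbits and zooms, with a timer restoring defaults after look input settles.
; Tick updates speed and acceleration text, while touch or R when tipped rights the car with input briefly locked, and RePosition stops it in place.
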(event `self.ReceiveTick`
  (params (DeltaSeconds :type "Float (single-precision)"))
  (`self.Update_Speed_String`))

(event `InputAxis|MoveRight`
  (params (AxisValue :type "Float (single-precision)"))
  (bind _simplewheeledvehiclemovement (`self.SimpleWheeledVehicleMovement`))
  (bind _steer_change_speed (`self.Steer_Change_Speed`))
  ;[1 0.9297 0] RIGHT / LEFT
  (bind _output_get (set `self.Steer_Angle_Curr` (select `bool` (`self.Upend`) :`false` (`KismetMathLibrary.FInterpTo` (`self.Steer_Angle_Curr`) (* AxisValue (* (`self.Steer_Angle_Max`) (`CurveFloat.GetFloatValue` (`self.Steering_Curve`) (`self.Curr_Car_Speed`)))) (`GameplayStatics.GetWorldDeltaSeconds`) (select `bool` (== AxisValue 0.0) :`false` _steer_change_speed :`true` (* _steer_change_speed 5.0))))))
  (`SimpleWheeledVehicleMovementComponent.SetSteerAngle` _simplewheeledvehiclemovement _output_get 0)
  (`SimpleWheeledVehicleMovementComponent.SetSteerAngle` _simplewheeledvehiclemovement _output_get 1))

(event `InputAxis|MoveForward`
  (params (AxisValue :type "Float (single-precision)"))
  (bind _simplewheeledvehiclemovement (`self.SimpleWheeledVehicleMovement`))
  (bind _returnvalue (select `bool` (> (`self.Curr_Car_Speed`) (`self.Max_Speed`)) :`false` (* (select `bool` (`self.Upend`) :`false` AxisValue) (`self.Throttle_Max`)) :`true` 1.0))
  ;[0 1 0.1831] FORWARD
  (`/Engine/EditorBlueprintResources/StandardMacros.CompareFloat` AxisValue
    (:`>`
      _)
    (:`==`
      (`|ExecutionSequence`
        (:`then_0`
          _)
        (:`then_1`
          (goto _label :!via `Reset`))))
    (:`<`
      (`self.Stop` AxisValue :!label _label)))
  (`SimpleWheeledVehicleMovementComponent.SetDriveTorque` _simplewheeledvehiclemovement _returnvalue 0)
  (`SimpleWheeledVehicleMovementComponent.SetDriveTorque` _simplewheeledvehiclemovement _returnvalue 1)
  (if (`self.4WD`)
    (`SimpleWheeledVehicleMovementComponent.SetDriveTorque` _simplewheeledvehiclemovement _returnvalue 2)
    (`SimpleWheeledVehicleMovementComponent.SetDriveTorque` _simplewheeledvehiclemovement _returnvalue 3)))

(event `InputAction|Handbrake`
  (params (Key :type "Key Structure"))
  (bind _simplewheeledvehiclemovement (`self.SimpleWheeledVehicleMovement`))
  ;[1 0 0.05503] BREAK
  (:`Pressed`
    (`SimpleWheeledVehicleMovementComponent.SetBrakeTorque` _simplewheeledvehiclemovement 2000.0 2)
    (`SimpleWheeledVehicleMovementComponent.SetBrakeTorque` _simplewheeledvehiclemovement 2000.0 3))
  (:`Released`
    (`SimpleWheeledVehicleMovementComponent.SetBrakeTorque` _simplewheeledvehiclemovement 0.0 2)
    (`SimpleWheeledVehicleMovementComponent.SetBrakeTorque` _simplewheeledvehiclemovement 0.0 3)))

(event `InputAxis|LookRight`
  (params (AxisValue :type "Float (single-precision)"))
  ;[1 1 1] MOUSE & Camera
  (`SceneComponent.K2_AddRelativeRotation` (`self.SpringArm`) (`KismetMathLibrary.MakeRotator` 0.0 0.0 (* AxisValue 5.0)) false false)
  (if (== (`self.Curr_Spring_Arm_Rot`) (`SceneComponent.RelativeRotation` (`self.SpringArm`)) :`ErrorTolerance` 0.2) :!label _label_2
    (`/Engine/EditorBlueprintResources/StandardMacros.DoOnce` false :!label _label_3
      (:`Completed`
        (bind _returnvalue (`KismetSystemLibrary.K2_SetTimerDelegate` (delegate `Set_Camera_Rot_Loc`) 2.0))))
    (else
      (set `self.Curr_Spring_Arm_Rot` (`SceneComponent.RelativeRotation` (`self.SpringArm`)))
      (`KismetSystemLibrary.K2_ClearAndInvalidateTimerHandle` _returnvalue)
      (`KismetSystemLibrary.K2_PauseTimerHandle` _returnvalue)
      (goto _label_3 :!via `Reset`))))

(event `InputAxis|LookUp`
  (params (AxisValue :type "Float (single-precision)"))
  ;[1 1 1] MOUSE & Camera
  (`SceneComponent.K2_AddRelativeRotation` (`self.SpringArm`) (`KismetMathLibrary.MakeRotator` 0.0 (* AxisValue 5.0)) false false)
  (goto _label_2))

(event `InputAxis|Scroll_UP`
  (params (AxisValue :type "Float (single-precision)"))
  (bind _springarm (`self.SpringArm`))
  ;[1 1 1] MOUSE & Camera
  (set `SpringArmComponent.TargetArmLength` (+ (* (`self.GetInputAxisKeyValue`) 10.0) (`SpringArmComponent.TargetArmLength` _springarm)) _springarm)
  (if (== (`self.Curr_Spring_Arm_Length`) (`SpringArmComponent.TargetArmLength` (`self.SpringArm`)))
    (goto _label_3)
    (else
      (set `self.Curr_Spring_Arm_Length` (`SpringArmComponent.TargetArmLength` (`self.SpringArm`)))
      (`KismetSystemLibrary.K2_ClearAndInvalidateTimerHandle` (stale `InputAxis|LookRight` _returnvalue))
      (`KismetSystemLibrary.K2_PauseTimerHandle` (stale `InputAxis|LookRight` _returnvalue))
      (goto _label_3 :!via `Reset`))))

(event `Set_Camera_Rot_Loc`
  ;[1 1 1] MOUSE & Camera
  (if (== (`self.Curr_Spring_Arm_Rot`) (`SceneComponent.RelativeRotation` (`self.SpringArm`)) :`ErrorTolerance` 0.2)
    (if (== (`self.Curr_Spring_Arm_Length`) (`SpringArmComponent.TargetArmLength` (`self.SpringArm`)))
      (`SceneComponent.K2_SetRelativeRotation` (`self.SpringArm`) (`self.Default_Spring_Arm_Rot`) false false)
      (set `SpringArmComponent.TargetArmLength` (`self.Default_Spring_Arm_Length`) (`self.SpringArm`)))))

(event `self.SkeletalMesh.OnInputTouchBegin`
  (params (FingerIndex :type "ETouchIndex Enum" :default "Touch1") (TouchedComponent :type "PrimitiveComponent Object Reference"))
  (bind (_returnvalue_x _returnvalue_y _returnvalue_z) (`KismetMathLibrary.BreakVector` (`self.K2_GetActorLocation`)))
  (bind (_returnvalue_roll _returnvalue_pitch _returnvalue_yaw) (`KismetMathLibrary.BreakRotator` (`self.K2_GetActorRotation`)))
  (bind _returnvalue (`GameplayStatics.GetPlayerController` 0))
  (bind _returnvalue_2 (`GameplayStatics.GetPlayerController` 0))
  (bind _simplewheeledvehiclemovement (`self.SimpleWheeledVehicleMovement`))
  ;[1 0.586 0.1692] REPOS
  (`/Engine/EditorBlueprintResources/StandardMacros.DoOnce` false :!label _label_4
    (:`Completed`
      (set `self.Upend` true)
      (set `PlayerController.bEnableTouchEvents` false _returnvalue)
      (set `PlayerController.bEnableClickEvents` false _returnvalue)
      (`self.DisableInput` _returnvalue)
      (`SimpleWheeledVehicleMovementComponent.SetDriveTorque` _simplewheeledvehiclemovement 0.0 0)
      (`SimpleWheeledVehicleMovementComponent.SetDriveTorque` _simplewheeledvehiclemovement 0.0 1)
      (`SimpleWheeledVehicleMovementComponent.SetDriveTorque` _simplewheeledvehiclemovement 0.0 2)
      (`SimpleWheeledVehicleMovementComponent.SetDriveTorque` _simplewheeledvehiclemovement 0.0 3)
      (`SimpleWheeledVehicleMovementComponent.SetSteerAngle` _simplewheeledvehiclemovement 0.0 0)
      (`SimpleWheeledVehicleMovementComponent.SetSteerAngle` _simplewheeledvehiclemovement 0.0 1)
      (`self.K2_SetActorLocationAndRotation` (`KismetMathLibrary.MakeVector` _returnvalue_x _returnvalue_y (+ _returnvalue_z 100.0)) (`KismetMathLibrary.MakeRotator` 0.0 0.0 _returnvalue_yaw) false true)
      (`PrimitiveComponent.AddImpulse` (`MovementComponent.UpdatedPrimitive` (`self.SimpleWheeledVehicleMovement`)) (* (`self.GetVelocity` (`GameplayStatics.GetPlayerPawn` 0)) -1) "None" true)
      (`KismetSystemLibrary.Delay` 3.0)
      (set `PlayerController.bEnableTouchEvents` true _returnvalue_2)
      (set `PlayerController.bEnableClickEvents` true _returnvalue_2)
      (`self.EnableInput` _returnvalue_2)
      (set `self.Upend` false)
      (`KismetSystemLibrary.Delay` 0.5)
      (goto _label_4 :!via `Reset`))))

(event `Key|R`
  (params (Key :type "Key Structure"))
  (bind (_returnvalue_x _returnvalue_y _returnvalue_z) (`KismetMathLibrary.BreakVector` (`self.GetActorUpVector`)))
  ;[1 0.586 0.1692] REPOS
  (:`Pressed`
    (if (or (> (`KismetMathLibrary.Abs` _returnvalue_y) 0.6) (< (`KismetMathLibrary.Abs` _returnvalue_z) 0.65))
      (goto _label_4))))

(event `RePosition`
  (bind _returnvalue (`GameplayStatics.GetPlayerController` 0))
  (bind _returnvalue_2 (`GameplayStatics.GetPlayerController` 0))
  (bind _simplewheeledvehiclemovement (`self.SimpleWheeledVehicleMovement`))
  ;[1 0.586 0.1692] REPOS
  (set `PlayerController.bEnableTouchEvents` false _returnvalue_2)
  (set `PlayerController.bEnableClickEvents` false _returnvalue_2)
  (`self.DisableInput` _returnvalue_2)
  (set `self.Upend` true)
  (`SimpleWheeledVehicleMovementComponent.SetDriveTorque` _simplewheeledvehiclemovement 0.0 0)
  (`SimpleWheeledVehicleMovementComponent.SetDriveTorque` _simplewheeledvehiclemovement 0.0 1)
  (`SimpleWheeledVehicleMovementComponent.SetDriveTorque` _simplewheeledvehiclemovement 0.0 2)
  (`SimpleWheeledVehicleMovementComponent.SetDriveTorque` _simplewheeledvehiclemovement 0.0 3)
  (`SimpleWheeledVehicleMovementComponent.SetSteerAngle` _simplewheeledvehiclemovement 0.0 0)
  (`SimpleWheeledVehicleMovementComponent.SetSteerAngle` _simplewheeledvehiclemovement 0.0 1)
  (`PrimitiveComponent.AddImpulse` (`MovementComponent.UpdatedPrimitive` (`self.SimpleWheeledVehicleMovement`)) (* (`self.GetVelocity` (`GameplayStatics.GetPlayerPawn` 0)) -1) "None" true)
  (`KismetSystemLibrary.Delay` 1.5)
  (set `PlayerController.bEnableTouchEvents` true _returnvalue)
  (set `PlayerController.bEnableClickEvents` true _returnvalue)
  (`self.EnableInput` _returnvalue)
  (set `self.Upend` false))

(fn `Stop_Car`
  (bind _simplewheeledvehiclemovement (`self.SimpleWheeledVehicleMovement`))
  (bind _simplewheeledvehiclemovement_2 (`self.SimpleWheeledVehicleMovement`))
  (`SimpleWheeledVehicleMovementComponent.SetBrakeTorque` _simplewheeledvehiclemovement 2000.0 2)
  (`SimpleWheeledVehicleMovementComponent.SetBrakeTorque` _simplewheeledvehiclemovement 2000.0 3)
  (`SimpleWheeledVehicleMovementComponent.SetBrakeTorque` _simplewheeledvehiclemovement_2 0.0 2)
  (`SimpleWheeledVehicleMovementComponent.SetBrakeTorque` _simplewheeledvehiclemovement_2 0.0 3))

(fn `Update_Speed_String`
  ;[1 1 1] Setup String for Speed
  (set `self.Curr_Car_Acc` (`self.Curr_Car_Acceleration`))
  (set `self.Curr_Car_Speed_Mph` (`self.Curr_Car_Speed`))
  (set `self.Curr_Speed_Mph_Text` (`KismetTextLibrary.Conv_StringToText` (`self.Cut_Speed_String` (`self.Curr_Car_Speed_Mph`) "." 1)))
  (set `self.Curr_Acc_Mph_Text` (`KismetTextLibrary.Conv_StringToText` (`self.Cut_Speed_String` (`self.Curr_Car_Acc`) "." 1)))
  (set `self.Curr_Speed_Percent` (/ (`self.Curr_Car_Speed_Mph`) (`self.Max_Speed`))))

(fn `UserConstructionScript`)