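; Race checkpoint actor that detects cars crossing it in the correct order and direction.
; Checkpoint 0 starts with every BPC_Car's display name; others receive names through an add-car event.
; On overlap, a listed car moving along the arrow is removed and CheckPointCleared is called with the next index and car name.
; Construction sizes the trigger and sets the index labels; spline-linking logic to the next checkpoint is disconnected.
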(event `Activate_First_Checkpoint`
  ;[1 1 1] Begin Play     Activate Checkpoint 0
  (if (== (`self.Checkpoint_Index`) 0)
    (bind _outactors (`GameplayStatics.GetAllActorsOfClass` "/Game/03_Car_Class/BPC_Car.BPC_Car_C"))
    (for _array_element _outactors
      (if (`KismetMathLibrary.ClassIsChildOf` (`GameplayStatics.GetObjectClass` _array_element) "/Game/03_Car_Class/BPC_Car.BPC_Car_C")
        (`KismetArrayLibrary.Array_AddUnique` (`self.Cars_Display_Names_Arr`) (`KismetSystemLibrary.GetDisplayName` _array_element))))))

(event `Add_Car_to_Next_Checkpoint_Collision`
  (params (Car_Name :type "String (by ref)"))
  (`KismetArrayLibrary.Array_AddUnique` (`self.Cars_Display_Names_Arr`) Car_Name))

(event `self.Trigger.OnComponentBeginOverlap`
  (params (OverlappedComponent :type "PrimitiveComponent Object Reference") (OtherActor :type "Actor Object Reference") (OtherComp :type "PrimitiveComponent Object Reference") (OtherBodyIndex :type Integer) (bFromSweep :type Boolean) (SweepResult :type "HitResult Structure (by ref)"))
  (bind _returnvalue (`KismetSystemLibrary.GetDisplayName` OtherActor))
  (bind _checkpoint_index (`self.Checkpoint_Index`))
  (if (`KismetMathLibrary.ClassIsChildOf` (`GameplayStatics.GetObjectClass` OtherActor) "/Game/03_Car_Class/BPC_Car.BPC_Car_C")
    (if (> (`KismetMathLibrary.Dot_VectorVector` (`self.GetVelocity` OtherActor) (`KismetMathLibrary.Conv_RotatorToVector` (`SceneComponent.K2_GetComponentRotation` (`self.Arrow`)))) 0.0)
      (if (`KismetArrayLibrary.Array_Contains` (`self.Cars_Display_Names_Arr`) _returnvalue)
        (`KismetArrayLibrary.Array_RemoveItem` (`self.Cars_Display_Names_Arr`) _returnvalue)
        ;[0.5383 1 0.4202] Next Checkpoint
        (`self.CheckPoint_Cleared` _checkpoint_index (+ _checkpoint_index 1) _returnvalue)))))

(fn `UserConstructionScript`
  (`SceneComponent.SetWorldScale3D` (`self.Trigger`) (`KismetMathLibrary.MakeVector` 1.0 (* (`self.Scale`) 10.0) 15.0))
  (`TextRenderComponent.K2_SetText` (`self.Checkpoint_Text`) (`KismetTextLibrary.Conv_StringToText` (`KismetStringLibrary.Concat_StrStr` "Checkpoint   " (`KismetStringLibrary.Conv_IntToString` (`self.Checkpoint_Index`)))))
  (`TextRenderComponent.K2_SetText` (`self.Checkpoint_Text1`) (`KismetTextLibrary.Conv_StringToText` (`KismetStringLibrary.Concat_StrStr` "Checkpoint   " (`KismetStringLibrary.Conv_IntToString` (`self.Checkpoint_Index`)))))
  (bind _outactors (`GameplayStatics.GetAllActorsOfClass` "BP_CheckPoints_C")))