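; Race track manager that pushes track settings and medal times to the player controller, starts music and tracks car progress.
; Checkpoint events arm the next checkpoint for that car, update laps and trigger a restart on race completion.
; A fast timer adds interpolated current-spline distance (spline length minus position) to completed segments per car, feeding the player's total to the controller.
; A slower timer snaps the player's respawn location onto the checkpoint spline.
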(event `self.ReceiveBeginPlay`
  (bind _asin_game_player_controller (cast `/Game/00_InGame/InGame_PlayerController` (`GameplayStatics.GetPlayerController` 0)))
  (bind _output_get (set `self.InGame_Player_Controller` _asin_game_player_controller))
  (set `/Game/00_InGame/InGame_PlayerController.BP_Tracker` self _output_get)
  (`AudioComponent.Play` (`AmbientSound.AudioComponent` (`self.Level_Music`)) 0.0)
  (`self.Apply_Settings`)
  (`self.Checkpoints_Start`)
  (`KismetSystemLibrary.K2_SetTimerDelegate` (delegate `Update_Respawn_Loc`) 1.0 true)
  (bind _outactors (`GameplayStatics.GetAllActorsOfClass` "/Game/03_Car_Class/BPC_Car.BPC_Car_C"))
  (bind _output_get_2 (set `self.Cars_Array` _outactors))
  (for _array_element _output_get_2
    (`KismetArrayLibrary.Array_AddUnique` (`self.Cars_Display_Names_Array`) (`KismetSystemLibrary.GetDisplayName` _array_element))
    (`KismetArrayLibrary.Array_AddUnique` (`self.Cars_Names_Array`) (`/Game/03_Car_Class/BPC_Car.Car_Name` _array_element))
    ;[1 1 1] Distance
    (`KismetArrayLibrary.Array_Add` (`self.PerCar_Prev_Spline_Distance`))
    (`KismetArrayLibrary.Array_Add` (`self.PerCar_Current_Spline_Distance`))
    (`KismetArrayLibrary.Array_Add` (`self.PerCar_Covered_Distance`))
    (`KismetArrayLibrary.Array_Add` (`self.PerCar_Current_Checkpoint`)))
  (for _array_element_2 (`self.BP_Checkpoints`)
    (set `self.Track_Length_UNITS` (+ (`self.Track_Length_UNITS`) (`KismetMathLibrary.FTrunc` (`SplineComponent.GetSplineLength` (`/Game/00_InGame/BP_CheckPoints.Spline` _array_element_2))))))
  (set `self.Track_Length_Meters` (`/Game/00_InGame/BP_Meter_Conversion_MacroLib.UNITS_to_Meters` (`KismetMathLibrary.Conv_IntToDouble` (`self.Track_Length_UNITS`))))
  (`self.Start_Distance_Timer`))

(event `Update_Respawn_Loc`
  (bind _returnvalue (`GameplayStatics.GetPlayerPawn` 0))
  (bind (_returnvalue_location _returnvalue_rotation _returnvalue_scale) (`KismetMathLibrary.BreakTransform` (`self.GetTransform` _returnvalue)))
  (bind _output (`|GetArrayItem` (`self.PerCar_Current_Checkpoint`) (`KismetArrayLibrary.Array_Find` (`self.Cars_Display_Names_Array`) (`KismetSystemLibrary.GetDisplayName` (`GameplayStatics.GetPlayerPawn` 0)))))
  (set `/Game/00_InGame/InGame_PlayerController.Respawn_Loc` (`KismetMathLibrary.MakeTransform` (`SplineComponent.FindLocationClosestToWorldLocation` (select `bool` (`KismetSystemLibrary.IsValid` _output) :`false` (`/Game/00_InGame/BP_CheckPoints.Spline` (`|GetArrayItem` (`self.BP_Checkpoints`))) :`true` (`/Game/00_InGame/BP_CheckPoints.Spline` _output)) (`self.K2_GetActorLocation` _returnvalue) "World") _returnvalue_rotation _returnvalue_scale) (`self.InGame_Player_Controller`)))

(event `Apply_Settings`
  (bind _ingame_player_controller (`self.InGame_Player_Controller`))
  ;[1 1 1] Settings       Max Lap   Save Slot   Name Map
  (set `/Game/00_InGame/InGame_PlayerController.Max_Laps` (`self.Max_Laps`) _ingame_player_controller)
  (set `/Game/00_InGame/InGame_PlayerController.Save_Slot` (`self.Save_Game_Name`) _ingame_player_controller)
  (set `/Game/00_InGame/InGame_PlayerController.Name_Map` (`self.Name_Map`) _ingame_player_controller)
  (`self.Update_Times`)
  (`/Game/00_InGame/InGame_PlayerController.Start_Game_Setup` _ingame_player_controller))

(event `Checkpoints_Start`
  ;[1 1 1] Checkppoints   START
  (for (_array_element _array_index) (`self.BP_Checkpoints`)
    (set `/Game/00_InGame/BP_CheckPoints.Checkpoint_Index` _array_index _array_element)
    (add `/Game/00_InGame/BP_CheckPoints.CheckPoint_Cleared` _array_element (delegate `CheckPoint_Cleared`))
    (if (== (`/Game/00_InGame/BP_CheckPoints.Checkpoint_Index` _array_element) 0)
      (`/Game/00_InGame/BP_CheckPoints.Activate_First_Checkpoint` _array_element)))
  (set `self.Last_Checkpoint_Index` (`KismetArrayLibrary.Array_LastIndex` (`self.BP_Checkpoints`))))

(event `CheckPoint_Cleared`
  (params (Curr_CheckPoint :type Integer) (Next_CheckPoint :type Integer) (Add_Car_To_Collision :type String))
  (bind _ingame_player_controller (`self.InGame_Player_Controller`))
  ;[1 1 1] Checkppoints   START
  (set `self.Prev_Checkpoint_Index` (`self.Cur_Checkpoint_Index`))
  (set `self.Cur_Checkpoint_Index` Curr_CheckPoint)
  (set `self.Next_Checkpoint_Index` Next_CheckPoint)
  (set `self.Add_Car_Name_to_Collision` Add_Car_To_Collision)
  (`self.Lap_Check`)
  (if (`/Game/00_InGame/InGame_PlayerController.Race_Complete` _ingame_player_controller)
    (`/Game/00_InGame/InGame_PlayerController.Restart` _ingame_player_controller))
  ;[1 1 1] PREV SPLINE COVERED DISTANCE
  (set `self.Temp_Car_Index` (`KismetArrayLibrary.Array_Find` (`self.Cars_Display_Names_Array`) (`self.Add_Car_Name_to_Collision`)))
  (if (`KismetSystemLibrary.IsValid` (`|GetArrayItem` (`self.PerCar_Current_Checkpoint`) (`self.Temp_Car_Index`)))
    (`KismetArrayLibrary.Array_Set` (`self.PerCar_Prev_Spline_Distance`) (`self.Temp_Car_Index`) (+ (`/Game/00_InGame/BP_Meter_Conversion_MacroLib.UNITS_to_Meters` (`SplineComponent.GetSplineLength` (`/Game/00_InGame/BP_CheckPoints.Spline` (`|GetArrayItem` (`self.PerCar_Current_Checkpoint`) (`self.Temp_Car_Index`))))) (`|GetArrayItem` (`self.PerCar_Prev_Spline_Distance`) (`self.Temp_Car_Index`)))))
  (`KismetArrayLibrary.Array_Set` (`self.PerCar_Current_Checkpoint`) (`self.Temp_Car_Index`) (`|GetArrayItem` (`self.BP_Checkpoints`) (`self.Cur_Checkpoint_Index`))))

(event `Start_Distance_Timer`
  ;[1 1 1] CURRENT SPLINE COVERED DISTANCE
  (`KismetSystemLibrary.K2_SetTimerDelegate` (delegate `Distance_Timer`) 0.1 true))

(event `Distance_Timer`
  (bind _ingame_player_controller (`self.InGame_Player_Controller`))
  ;[1 1 1] CURRENT SPLINE COVERED DISTANCE
  (for (_array_element _array_index) (`self.Cars_Array`)
    (if (`KismetSystemLibrary.IsValid` (`|GetArrayItem` (`self.PerCar_Current_Checkpoint`) _array_index))
      (bind _newparam (`self.F_Current_Spline_Distance` _array_element (`/Game/00_InGame/BP_CheckPoints.Spline` (`|GetArrayItem` (`self.PerCar_Current_Checkpoint`) _array_index))))
      (`KismetArrayLibrary.Array_Set` (`self.PerCar_Current_Spline_Distance`) _array_index _newparam)
      (`KismetArrayLibrary.Array_Set` (`self.PerCar_Covered_Distance`) _array_index (+ (`|GetArrayItem` (`self.PerCar_Prev_Spline_Distance`) _array_index) (`|GetArrayItem` (`self.PerCar_Current_Spline_Distance`) _array_index)))
      (if (== (`KismetArrayLibrary.Array_Find` (`self.Cars_Display_Names_Array`) (`KismetSystemLibrary.GetDisplayName` (`GameplayStatics.GetPlayerPawn` 0))) _array_index)
        (set `/Game/00_InGame/InGame_PlayerController.Covered_Distance` (`|GetArrayItem` (`self.PerCar_Covered_Distance`) _array_index) _ingame_player_controller)
        (`/Game/00_InGame/InGame_PlayerController.Prev_Next_Cars_Distance` _ingame_player_controller)))))

(fn `F_Current_Spline_Distance`
  (params (Car_Target :type "Actor Object Reference") (Spline_Component :type "SplineComponent Object Reference") (Draw_Sphere :type Boolean))
  (returns (NewParam :type Integer))
  (locals (Prev_L :type "Vector Structure") (Next_L :type "Vector Structure"))
  (bind _returnvalue (`KismetMathLibrary.FTrunc` (`SplineComponent.FindInputKeyClosestToWorldLocation` Spline_Component (`self.K2_GetActorLocation` Car_Target))))
  (bind _returnvalue_2 (+ _returnvalue 1))
  (bind _returnvalue_3 (`KismetMathLibrary.Lerp` (`SplineComponent.GetDistanceAlongSplineAtSplinePoint` Spline_Component _returnvalue) (`SplineComponent.GetDistanceAlongSplineAtSplinePoint` Spline_Component _returnvalue_2) (/ (`KismetMathLibrary.VSize` (- (`SplineComponent.FindLocationClosestToWorldLocation` Spline_Component (`self.K2_GetActorLocation` Car_Target) "World") (`local.Prev_L`))) (`KismetMathLibrary.VSize` (- (`local.Next_L`) (`local.Prev_L`))))))
  (set `local.Prev_L` (`SplineComponent.GetLocationAtSplinePoint` Spline_Component _returnvalue "World"))
  (set `local.Next_L` (`SplineComponent.GetLocationAtSplinePoint` Spline_Component _returnvalue_2 "World"))
  (if Draw_Sphere
    (`KismetSystemLibrary.DrawDebugSphere` (`SplineComponent.GetLocationAtDistanceAlongSpline` Spline_Component _returnvalue_3 "World") 100.0 12 (struct :`R` 0.457007 :`G` 0.648313 :`B` 0.351178 :`A` 1.0) 0.1 1.0))
  (return (`KismetMathLibrary.FTrunc` (/ (/ (- (`SplineComponent.GetSplineLength` Spline_Component) _returnvalue_3) 100.0) 3.15))))

(fn `Lap_Check`
  ;[1 1 1] Start Race
  (if (and (== (`self.Prev_Checkpoint_Index`) 999) (== (`self.Cur_Checkpoint_Index`) 0) (== (`self.Next_Checkpoint_Index`) 1))
    (`/Game/00_InGame/BP_CheckPoints.Add_Car_to_Next_Checkpoint_Collision` (`|GetArrayItem` (`self.BP_Checkpoints`) (`self.Next_Checkpoint_Index`)) (`self.Add_Car_Name_to_Collision`))
    (else
      ;[1 1 1] Lap
      (if (and (== (`self.Prev_Checkpoint_Index`) (`self.Last_Checkpoint_Index`)) (== (`self.Cur_Checkpoint_Index`) 0) (== (`self.Next_Checkpoint_Index`) 1))
        (bind _is_race_complete (`self.Race_Complete_Check`))
        (if (not _is_race_complete)
          (`/Game/00_InGame/BP_CheckPoints.Add_Car_to_Next_Checkpoint_Collision` (`|GetArrayItem` (`self.BP_Checkpoints`) 1) (`self.Add_Car_Name_to_Collision`)))
        (`/Game/00_InGame/InGame_PlayerController.Update_Lap` (`self.InGame_Player_Controller`))
        (else
          ;[1 1 1] Last Checkpoint
          (if (and (== (`self.Cur_Checkpoint_Index`) (`self.Last_Checkpoint_Index`)) (> (`self.Next_Checkpoint_Index`) (`self.Last_Checkpoint_Index`)))
            (`/Game/00_InGame/BP_CheckPoints.Add_Car_to_Next_Checkpoint_Collision` (`|GetArrayItem` (`self.BP_Checkpoints`)) (`self.Add_Car_Name_to_Collision`))
            (else
              ;[1 1 1] Next Checkpoint
              (`/Game/00_InGame/BP_CheckPoints.Add_Car_to_Next_Checkpoint_Collision` (`|GetArrayItem` (`self.BP_Checkpoints`) (`self.Next_Checkpoint_Index`)) (`self.Add_Car_Name_to_Collision`))))))))
  (return))

(fn `Race_Complete_Check`
  (returns (Is_Race_Complete :type Boolean))
  (locals (Local_Complete :type Boolean))
  (bind _ingame_player_controller (`self.InGame_Player_Controller`))
  (bind _output_get (set `/Game/00_InGame/InGame_PlayerController.Race_Complete` (>= (`/Game/00_InGame/InGame_PlayerController.Actual_Lap` _ingame_player_controller) (`/Game/00_InGame/InGame_PlayerController.Max_Laps` _ingame_player_controller)) (`self.InGame_Player_Controller`)))
  (return _output_get))

(fn `Update_Times`
  (bind _ingame_player_controller (`self.InGame_Player_Controller`))
  (set `/Game/00_InGame/InGame_PlayerController.Gold_Time` (`self.Gold_Time`) _ingame_player_controller)
  (set `/Game/00_InGame/InGame_PlayerController.Silver_Time` (`self.Silver_Time`) _ingame_player_controller)
  (set `/Game/00_InGame/InGame_PlayerController.Bronze_Time` (`self.Bronze_Time`) _ingame_player_controller)
  (set `/Game/00_InGame/InGame_PlayerController.Default_Lap_Time` (`self.Default_Best_Lap`) _ingame_player_controller)
  (set `/Game/00_InGame/InGame_PlayerController.Default_Race_Time` (`self.Default_Best_Time`) _ingame_player_controller))

(fn `UserConstructionScript`)